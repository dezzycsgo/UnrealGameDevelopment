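; CustomPlayerStart is a team-tagged player start that stores a Team value (NoTeam, BlueTeam or RedTeam).
; Its construction script writes the team name to a TextRender component and colors it white, blue or red by team.
; A SetTeam event and a GetTeam function let other code assign and read the team.
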(event `/Game/l012809i/Blueprints/Interfaces/BPI-Teams.SetTeam`
  (params (Team :type "/Game/l012809i/Enums/E_Teams Enum" :default "NewEnumerator0"))
  (set `self.Team` Team))

(fn `GetTeam`
  (returns (Team :type "/Game/l012809i/Enums/E_Teams Enum"))
  (return (`self.Team`)))

(fn `UserConstructionScript`
  (bind _textrender (`self.TextRender`))
  (`TextRenderComponent.K2_SetText` _textrender (`KismetTextLibrary.Conv_StringToText` (`|GetEnumeratorNameAsString` (`self.Team`))))
  (`TextRenderComponent.SetTextRenderColor` _textrender (select `/Game/l012809i/Enums/E_Teams` (`self.Team`) :`NewEnumerator0` (`KismetMathLibrary.LinearColor_Quantize` (struct :`R` 1.0 :`G` 1.0 :`B` 1.0 :`A` 1.0)) :`NewEnumerator1` (`KismetMathLibrary.LinearColor_Quantize` (struct :`G` 0.155449 :`B` 1.0 :`A` 1.0)) :`NewEnumerator2` (`KismetMathLibrary.LinearColor_Quantize` (struct :`R` 0.375 :`B` 0.011932 :`A` 1.0)))))